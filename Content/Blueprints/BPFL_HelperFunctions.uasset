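; Blueprint function library of camera and vector helpers built on the first player's camera manager.
; Position and forward-vector getters feed two object-type line traces from the camera.
; The long trace takes caller-supplied types and returns impact point or trace end plus normal; the short WorldStatic trace returns impact normal or zero, with one-frame debug drawing.
; A separate helper gives the angle in degrees between direction vectors via arccosine of their dot product.
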(fn `GetCameraForwardVector`
  (returns (ForwardDir :type "Vector Structure"))
  (return (`SceneComponent.GetForwardVector` (`PlayerCameraManager.TransformComponent` (`GameplayStatics.GetPlayerCameraManager` null)))))

(fn `GetCameraLineTraceForward`
  (params (ObjectTypes :type "Array of EObjectTypeQuery Enum (by ref)"))
  (returns (LineTraceImpactOrEnd :type "Vector Structure") (LineTraceNormal :type "Vector Structure"))
  (bind _camera_position (`self.GetCameraPosition` null))
  (bind (_outhit _returnvalue) (`KismetSystemLibrary.LineTraceSingleForObjects` null _camera_position (+ _camera_position (* (`self.GetCameraForwardVector` null) 3000000.0)) ObjectTypes))
  (return (select `bool` _returnvalue :`false` (`.TraceEnd` (`GameplayStatics.BreakHitResult` _outhit)) :`true` (`.ImpactPoint` (`GameplayStatics.BreakHitResult` _outhit))) (`.Normal` (`GameplayStatics.BreakHitResult` _outhit))))

(fn `GetCameraLineTraceForwardImpactNormal`
  (returns (ImpactNormal :type "Vector Structure"))
  (bind _camera_position (`self.GetCameraPosition` null))
  (bind (_outhit _returnvalue) (`KismetSystemLibrary.LineTraceSingleForObjects` :`Start` _camera_position :`End` (+ _camera_position (* (`self.GetCameraForwardVector` null) 3000.0)) :`ObjectTypes` (`|MakeArray` "ObjectTypeQuery1" :!type "EObjectTypeQuery Enum") :`DrawDebugType` "ForOneFrame"))
  (return (select `bool` _returnvalue :`true` (`.ImpactNormal` (`GameplayStatics.BreakHitResult` _outhit)))))

(fn `GetCameraPosition`
  (returns (`Camera Position` :type "Vector Structure"))
  (return (`SceneComponent.K2_GetComponentLocation` (`PlayerCameraManager.TransformComponent` (`GameplayStatics.GetPlayerCameraManager` null)))))

(fn `GetVectorAngleDifference`
  (params (`Directional Vector 1` :type "Vector Structure") (DirectionalVector2 :type "Vector Structure"))
  (returns (AngleDifference :type "Float (double-precision)"))
  (return (`KismetMathLibrary.DegAcos` (`KismetMathLibrary.Dot_VectorVector` `Directional Vector 1` DirectionalVector2))))