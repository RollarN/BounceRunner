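; BPC_SelfLauncher is a first person character component that lets the player launch themselves while the character's OverlapChecker is touching something.
; Each key looks up its own up-vector alpha, which feeds the character's Launch along with a shared launch force.
; Overlaps enable launching, and a coyote timer delays disabling it after the last overlap ends.
; Failed attempts are buffered and fire on the next overlap if the key is still held or was pressed recently.
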(event `self.ReceiveBeginPlay`
  (bind (_asfirst_person_character _bsuccess) (cast `/Game/FirstPersonBP/Blueprints/FirstPersonCharacter` (`self.GetOwner`) :!pure true))
  (if _bsuccess
    (set `self.FirstPersonCharacter` _asfirst_person_character)
    (add `PrimitiveComponent.OnComponentBeginOverlap` (`/Game/FirstPersonBP/Blueprints/FirstPersonCharacter.OverlapChecker` (`self.FirstPersonCharacter`)) (delegate `CheckerBeginOverlap`))
    (add `PrimitiveComponent.OnComponentEndOverlap` (`/Game/FirstPersonBP/Blueprints/FirstPersonCharacter.OverlapChecker` (`self.FirstPersonCharacter`)) (delegate `Reset Launch Coyote Time`))
    (else
      (`KismetSystemLibrary.PrintString` "Spawners can only be placed on the First person character" true true (struct :`R` 1.0 :`A` 1.0))
      (`self.K2_DestroyComponent`))))

(event `CheckerBeginOverlap`
  (params (OverlappedComponent :type "PrimitiveComponent Object Reference") (OtherActor :type "Actor Object Reference") (OtherComp :type "PrimitiveComponent Object Reference") (OtherBodyIndex :type Integer) (bFromSweep :type Boolean) (SweepResult :type "HitResult Structure (by ref)"))
  (`KismetSystemLibrary.K2_ClearAndInvalidateTimerHandle` (`self.Launch Coyote Time Handle`))
  (set `self.CanLaunch` true)
  (if (or (`PlayerController.IsInputKeyDown` (`GameplayStatics.GetPlayerController` 0) (`self.BufferedLaunchKey`)) (< (- (`GameplayStatics.GetTimeSeconds`) (`self.BufferedLaunchSeconds`)) (`self.LaunchTimeBuffer`)))
    (`/Game/Blueprints/Interfaces/BPI_LaunchAble.Launch` (`self.FirstPersonCharacter`) (`self.GetUpVectorAlphaValueByKey` (`self.BufferedLaunchKey`)) (`self.LaunchForce`))))

(event `Reset Launch Coyote Time`
  (params (OverlappedComponent :type "PrimitiveComponent Object Reference") (OtherActor :type "Actor Object Reference") (OtherComp :type "PrimitiveComponent Object Reference") (OtherBodyIndex :type Integer))
  (`KismetSystemLibrary.K2_ClearAndInvalidateTimerHandle` (`self.Launch Coyote Time Handle`))
  (if (not (> (`KismetArrayLibrary.Array_Length` (`PrimitiveComponent.GetOverlappingComponents` (`/Game/FirstPersonBP/Blueprints/FirstPersonCharacter.OverlapChecker` (`self.FirstPersonCharacter`)))) 0))
    (bind _returnvalue (`KismetSystemLibrary.K2_SetTimerDelegate` (delegate `End Launch Coyote Time`) (`self.CoyoteTime`)))
    (set `self.Launch Coyote Time Handle` _returnvalue)))

(event `End Launch Coyote Time`
  (set `self.CanLaunch` false))

(fn `AttemptLaunchPlayer`
  (params (Key :type "Key Structure" :default "None"))
  (set `self.BufferedLaunchKey` (`local.Key`))
  (if (`self.CanLaunch`)
    (`/Game/Blueprints/Interfaces/BPI_LaunchAble.Launch` (`self.FirstPersonCharacter`) (`self.GetUpVectorAlphaValueByKey` (`local.Key`)) (`self.LaunchForce`))
    (else
      (set `self.BufferedLaunchSeconds` (`GameplayStatics.GetTimeSeconds`)))))

(fn `GetUpVectorAlphaValueByKey`
  (params (Key :type "Key Structure (by ref)"))
  (returns (UpVectorAlpha :type "Float (double-precision)"))
  (bind (_value _returnvalue) (`BlueprintMapLibrary.Map_Find` (`self.UpVectorAlphaValueDictionary`) Key))
  (if _returnvalue
    (return _value)
    (else
      (`KismetSystemLibrary.PrintString` "Key not found in dictionary"))))