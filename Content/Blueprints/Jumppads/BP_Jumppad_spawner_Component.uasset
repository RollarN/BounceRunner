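; Player component for the first-person character that previews and places jump pads, destroying itself on any other owner.
; BeginPlay pre-spawns a pool of pads out of sight and a dummy visualizer, which Tick aligns to the camera's world-static trace.
; Activation recycles pads round-robin, copying the preview's transform, material and selected up-vector alpha.
; A test variant drops a pad at the owner's location.
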(event `self.ReceiveBeginPlay`
  (if (== (`GameplayStatics.GetObjectClass` (`self.GetOwner`)) "/Game/FirstPersonBP/Blueprints/FirstPersonCharacter.FirstPersonCharacter_C")
    (for _ (range (`self.MaxAmountOfJumpPads`))
      (bind _returnvalue (`|SpawnActorFromClass` "/Game/Blueprints/Jumppads/BP_Jumppad.BP_Jumppad_C" (`KismetMathLibrary.MakeTransform` (0.0 0.0 -100000.0)) "Undefined" "OverrideRootScale" null null))
      (`KismetArrayLibrary.Array_Add` (`self.JumpPadPool`) _returnvalue))
    (bind _returnvalue_2 (`|SpawnActorFromClass` "/Game/Blueprints/Jumppads/BP_Jumppad_Dummy.BP_Jumppad_Dummy_C" (`KismetMathLibrary.MakeTransform` (0.0 0.0 0.0)) "AlwaysSpawn" "OverrideRootScale" null null))
    (set `self.JumpPadVisualizer` _returnvalue_2)
    (`self.Toggle Jump Pad Visualization` false)
    (`self.Update Up Vector Alpha` 0)
    (else
      (`KismetSystemLibrary.PrintString` "Spawners can only be placed on the First person character" true true (struct :`R` 1.0 :`A` 1.0))
      (`self.K2_DestroyComponent`))))

(event `self.ReceiveTick`
  (params (DeltaSeconds :type "Float (single-precision)"))
  (bind (_linetraceimpactorend _linetracenormal) (`/Game/Blueprints/BPFL_HelperFunctions.GetCameraLineTraceForward` (`|MakeArray` "ObjectTypeQuery1" :!type "EObjectTypeQuery Enum")))
  (`Actor.K2_SetActorLocationAndRotation` (`self.JumpPadVisualizer`) _linetraceimpactorend (`KismetMathLibrary.FindLookAtRotation` (`KismetMathLibrary.Vector_Zero`) _linetracenormal) false false))

(fn `ActivateJumpPad`
  (locals (ActivatedJumpPad :type "/Game/Blueprints/Jumppads/BP_Jumppad Object Reference"))
  (bind (_returnvalue_location _returnvalue_rotation) (`KismetMathLibrary.BreakTransform` (`SceneComponent.K2_GetComponentToWorld` (`/Game/Blueprints/Jumppads/BP_Jumppad.DefaultSceneRoot` (`self.JumpPadVisualizer`)))))
  (set `self.JumpPadPoolIndex` (mod (+ (`self.JumpPadPoolIndex`) 1) (`self.MaxAmountOfJumpPads`)))
  (bind _output_get (set `local.ActivatedJumpPad` (`|GetArrayItem` (`self.JumpPadPool`) (`self.JumpPadPoolIndex`))))
  (set `/Game/Blueprints/Jumppads/BP_Jumppad.UpVectorAlpha` (`self.UpVectorAlpha`) _output_get)
  (`Actor.K2_SetActorLocationAndRotation` (`local.ActivatedJumpPad`) _returnvalue_location _returnvalue_rotation false false)
  (`PrimitiveComponent.SetMaterial` (`/Game/Blueprints/Jumppads/BP_Jumppad.StaticMesh` (`local.ActivatedJumpPad`)) 0 (`PrimitiveComponent.GetMaterial` (`/Game/Blueprints/Jumppads/BP_Jumppad.StaticMesh` (`self.JumpPadVisualizer`)) 0)))

(fn `GetLineTraceForwardForDummyNormal`
  (returns (LineTraceImpactNormal :type "Vector Structure"))
  (bind (_outhit _returnvalue) (`KismetSystemLibrary.LineTraceSingleForObjects` :`Start` (`/Game/Blueprints/BPFL_HelperFunctions.GetCameraPosition`) :`End` (+ (`/Game/Blueprints/BPFL_HelperFunctions.GetCameraPosition`) (* (`/Game/Blueprints/BPFL_HelperFunctions.GetCameraForwardVector`) 300000.0)) :`ObjectTypes` (`|MakeArray` "ObjectTypeQuery5" :!type "EObjectTypeQuery Enum") :`bIgnoreSelf` false :`DrawTime` 50.0))
  (return (select `bool` _returnvalue :`false` (0.0 0.0 1.0) :`true` (`.ImpactNormal` (`GameplayStatics.BreakHitResult` _outhit)))))

(fn `GetLineTraceForwardForDummyPlane`
  (returns (LineTraceImpactPointOrEnd :type "Vector Structure"))
  (bind _camera_position (`/Game/Blueprints/BPFL_HelperFunctions.GetCameraPosition`))
  (bind (_outhit _returnvalue) (`KismetSystemLibrary.LineTraceSingleForObjects` :`Start` _camera_position :`End` (+ _camera_position (* (`/Game/Blueprints/BPFL_HelperFunctions.GetCameraForwardVector`) 3000.0)) :`ObjectTypes` (`|MakeArray` "ObjectTypeQuery5" :!type "EObjectTypeQuery Enum") :`bIgnoreSelf` false :`DrawTime` 50.0))
  (return (select `bool` _returnvalue :`false` (`.TraceEnd` (`GameplayStatics.BreakHitResult` _outhit)) :`true` (`.ImpactPoint` (`GameplayStatics.BreakHitResult` _outhit)))))

(fn `Test Instant Activate Jump Pad (For Testing the Instant-launch)`
  (locals (ActivatedJumpPad :type "/Game/Blueprints/Jumppads/BP_Jumppad Object Reference"))
  (set `self.JumpPadPoolIndex` (mod (+ (`self.JumpPadPoolIndex`) 1) (`self.MaxAmountOfJumpPads`)))
  (bind _output_get (set `local.ActivatedJumpPad` (`|GetArrayItem` (`self.JumpPadPool`) (`self.JumpPadPoolIndex`))))
  (set `/Game/Blueprints/Jumppads/BP_Jumppad.UpVectorAlpha` (`self.UpVectorAlpha`) _output_get)
  (`Actor.K2_SetActorLocationAndRotation` :`self` (`local.ActivatedJumpPad`) :`NewLocation` (`Actor.K2_GetActorLocation` (`self.GetOwner`)))
  (`PrimitiveComponent.SetMaterial` (`/Game/Blueprints/Jumppads/BP_Jumppad.StaticMesh` (`local.ActivatedJumpPad`)) 0 (`PrimitiveComponent.GetMaterial` (`/Game/Blueprints/Jumppads/BP_Jumppad.StaticMesh` (`self.JumpPadVisualizer`)) 0)))

(fn `Toggle Jump Pad Visualization`
  (params (KeyDown :type Boolean))
  (`SceneComponent.SetVisibility` (`/Game/Blueprints/Jumppads/BP_Jumppad.DefaultSceneRoot` (`self.JumpPadVisualizer`)) (`local.KeyDown`) true))

(fn `Update Up Vector Alpha`
  (params (`Input Int` :type Integer))
  (locals (NewLocalVar_0 :type "Color Structure"))
  (set `self.UpVectorAlphaIndex` (`KismetMathLibrary.Clamp` (+ `Input Int` (`self.UpVectorAlphaIndex`)) 0 (- (`KismetArrayLibrary.Array_Length` (`self.UpVectorAlphaValues`)) 1)))
  (set `self.UpVectorAlpha` (`|GetArrayItem` (`self.UpVectorAlphaValues`) (`self.UpVectorAlphaIndex`)))
  (`PrimitiveComponent.SetMaterial` (`/Game/Blueprints/Jumppads/BP_Jumppad.StaticMesh` (`self.JumpPadVisualizer`)) 0 (`|GetArrayItem` (`self.JumpPadMaterials`) (`self.UpVectorAlphaIndex`))))